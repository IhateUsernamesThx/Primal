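; Music manager actor that fades in idle music at BeginPlay and changes it as the player character enters or leaves trigger volumes.
; Entering the boss room fades out idle music, then starts or restores boss music after a delay; leaving reverses this.
; A ShouldPlay flag rechecked after each delay guards against quick re-entry or exit.
; The bear cave trigger only lowers idle music while the player is inside.
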(event OnComponentBeginOverlap(BossRoom)
  (params (OverlappedComponent :type Primitive%20Component%20Object%20Reference) (OtherActor :type Actor%20Object%20Reference) (OtherComp :type Primitive%20Component%20Object%20Reference) (OtherBodyIndex :type Integer) (bFromSweep :type Boolean) (SweepResult :type Hit%20Result%20Structure%20%28by%20ref%29))
  (bind _bossmusic (Variables|Default|GetBossMusic))
  (Utilities|Casting|CastToBP_ThirdPersonCharacter OtherActor)
  (Variables|Default|SetShouldPlay true)
  (Audio|Components|Audio|AdjustVolume (Variables|Default|GetIdleMusic) 1.0 0.0 "Linear" :!class /Script/Engine.AudioComponent)
  (Utilities|FlowControl|Delay 1.0)
  (if (Variables|Default|GetShouldPlay)
    (if (Audio|Components|Audio|IsPlaying _bossmusic)
      (Audio|Components|Audio|AdjustVolume _bossmusic 0.0 0.5 "Linear" :!class /Script/Engine.AudioComponent)
      (else
        (Audio|Components|Audio|Play _bossmusic 0.0)))))

(event OnComponentEndOverlap(BossRoom)
  (params (OverlappedComponent :type Primitive%20Component%20Object%20Reference) (OtherActor :type Actor%20Object%20Reference) (OtherComp :type Primitive%20Component%20Object%20Reference) (OtherBodyIndex :type Integer))
  (Utilities|Casting|CastToBP_ThirdPersonCharacter OtherActor)
  (Variables|Default|SetShouldPlay false)
  (Audio|Components|Audio|AdjustVolume (Variables|Default|GetBossMusic) 3.0 0.0 "Linear" :!class /Script/Engine.AudioComponent)
  (Utilities|FlowControl|Delay 3.0)
  (if (not (Variables|Default|GetShouldPlay))
    (Audio|Components|Audio|AdjustVolume (Variables|Default|GetIdleMusic) 2.0 0.5 "Linear" :!class /Script/Engine.AudioComponent)))

(event OnComponentBeginOverlap(BearCave)
  (params (OverlappedComponent :type Primitive%20Component%20Object%20Reference) (OtherActor :type Actor%20Object%20Reference) (OtherComp :type Primitive%20Component%20Object%20Reference) (OtherBodyIndex :type Integer) (bFromSweep :type Boolean) (SweepResult :type Hit%20Result%20Structure%20%28by%20ref%29))
  (Utilities|Casting|CastToBP_ThirdPersonCharacter OtherActor)
  (Audio|Components|Audio|AdjustVolume (Variables|Default|GetIdleMusic) 2.0 0.1 "Linear" :!class /Script/Engine.AudioComponent))

(event OnComponentEndOverlap(BearCave)
  (params (OverlappedComponent :type Primitive%20Component%20Object%20Reference) (OtherActor :type Actor%20Object%20Reference) (OtherComp :type Primitive%20Component%20Object%20Reference) (OtherBodyIndex :type Integer))
  (Utilities|Casting|CastToBP_ThirdPersonCharacter OtherActor)
  (Audio|Components|Audio|AdjustVolume (Variables|Default|GetIdleMusic) 2.0 0.5 "Linear" :!class /Script/Engine.AudioComponent))

(event EventBeginPlay
  (Audio|Components|Audio|FadeIn (Variables|Default|GetIdleMusic) 2.0 1.0 0.0 "Linear" :!class /Script/Engine.AudioComponent))

(fn ConstructionScript)