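; BP_OwlManager periodically plays an owl hoot from a randomly chosen owl actor.
; On BeginPlay it starts a looping timer with a random interval, rolled once and then kept for every repeat.
; Each tick of the timer plays the OwlHoot of a random OutActors entry and prints an actor name from a separate random pick, so the printed owl can differ from the one heard.
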(event Custom|PlaySound
  (bind _out_actors (Variables|Default|GetOut%20Actors))
  (bind _returnvalue (Utilities|Array|Length _out_actors))
  (bind _returnvalue_2 (- _returnvalue 1))
  (bind _returnvalue_3 (Math|Random|RandomIntegerinRange 0 _returnvalue_2))
  (bind _output (Utilities|Array|Get(acopy) _out_actors _returnvalue_3))
  (Audio|Components|Audio|Play (Variables|/Game/Audio/BP_OwlHoot.BP_OwlHoot_C|GetOwlHoot _output) 0.0)
  (Development|PrintString (Utilities|GetDisplayName _output)))

(event EventBeginPlay
  (Utilities|Time|SetTimerbyEvent (delegate Custom|PlaySound) (Math|Random|RandomFloatinRange 5.0 15.0) true))

(fn ConstructionScript)