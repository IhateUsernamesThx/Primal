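; BP_Raptor is a raptor AI pawn that wanders endlessly around the navmesh.
; On BeginPlay it starts the Roam loop and toggles physical animation through ACPhysicalAnimComp.
; Roam uses AI MoveTo toward a random navigable point within a randomized radius of the mesh's current location, then calls itself again after a short delay on either success or failure.
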(event Custom|Roam
  (bind _randomlocation (Class|NavigationSystemV1|GetRandomLocationinNavigableRadius (Transformation|GetWorldLocation (Variables|Character|GetMesh)) (Math|Random|RandomFloatinRange 3e+02 1.5e+03) 0 0))
  (AI|AIMoveTo self _randomlocation 0 15.0 false
    (:OnSuccess
      _)
    (:OnFail
      _))
  (Utilities|FlowControl|Delay 0.2)
  (CallFunction|Roam))

(event EventBeginPlay
  (CallFunction|Roam)
  (Default|TogglePhysicalAnimation (Variables|Default|GetAC_PhysicalAnimComp)))

(fn ConstructionScript)